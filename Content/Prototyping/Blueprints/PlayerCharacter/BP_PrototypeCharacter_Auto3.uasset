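; Prototype player character that previews building placement on build plots under the cursor.
; On IA_Target, a complex Visibility trace from the cursor finds a static mesh component; on a BPA_BuildPlot, it adds a component with the preview mesh and material, using the impact normal as relative transform.
; Targeting an existing preview mesh only prints a placeholder for the unimplemented build step, and misses print debug messages.
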(event `EnhancedInput|/Game/Prototyping/InputActions/IA_Target`
  (params (ActionValue :type Boolean) (ElapsedSeconds :type "Float (double-precision)") (TriggeredSeconds :type "Float (double-precision)") (InputAction :type "InputAction Object Reference" :default "/Game/Prototyping/InputActions/IA_Target.IA_Target"))
  (bind (_bblockinghit _binitialoverlap _time _distance _location _impactpoint _normal _impactnormal _physmat _hitactor _hitcomponent) (`GameplayStatics.BreakHitResult` (`PlayerController.GetHitResultUnderCursorByChannel` (`GameplayStatics.GetPlayerController` 0) "TraceTypeQuery1" true)))
  (:`Triggered`
    (bind _asstatic_mesh_component (cast `StaticMeshComponent` _hitcomponent)
      (:`then`
        (if (== (`StaticMeshComponent.StaticMesh` _asstatic_mesh_component) (`self.PreviewStaticMesh`))
          (`KismetSystemLibrary.PrintString` "Put build functinonality here")
          (else
            (bind _asbpa_build_plot (cast `/Game/Prototyping/Blueprints/Building/BPA_BuildPlot` _hitactor)
              (:`then`
                (bind _returnvalue (`AddComponent|NODE_AddStaticMeshComponent-0` :`self` _asbpa_build_plot :`RelativeTransform` (`KismetMathLibrary.Conv_VectorToTransform` _impactnormal)))
                (`StaticMeshComponent.SetStaticMesh` _returnvalue (`self.PreviewStaticMesh`))
                (`PrimitiveComponent.SetMaterial` _returnvalue 0 "/Game/Prototyping/Blueprints/Building/M_BuildPreview.M_BuildPreview"))
              (:`CastFailed`
                (`KismetSystemLibrary.PrintString` "Miss"))))))
      (:`CastFailed`
        (`KismetSystemLibrary.PrintString` "wtf?")))))

(fn `UserConstructionScript`)