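; Prototype player character that tests placing build-preview meshes on build plots under the mouse cursor.
; The IA_Target input runs a cursor visibility trace and prints a debug message if the hit actor casts to StaticMesh.
; Otherwise, a BPA_BuildPlot hit gains a cube mesh component with a preview material, its relative transform converted from the impact normal rather than the hit location.
; Other hits print a miss.
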(event `EnhancedInput|/Game/Prototyping/InputActions/IA_Target`
  (params (ActionValue :type Boolean) (ElapsedSeconds :type "Float (double-precision)") (TriggeredSeconds :type "Float (double-precision)") (InputAction :type "InputAction Object Reference" :default "/Game/Prototyping/InputActions/IA_Target.IA_Target"))
  (bind (_bblockinghit _binitialoverlap _time _distance _location _impactpoint _normal _impactnormal _physmat _hitactor) (`GameplayStatics.BreakHitResult` (`PlayerController.GetHitResultUnderCursorByChannel` (`GameplayStatics.GetPlayerController` 0) "TraceTypeQuery1" true)))
  (:`Triggered`
    (cast `StaticMesh` _hitactor
      (:`then`
        (`KismetSystemLibrary.PrintString` "Hello"))
      (:`CastFailed`
        (bind _asbpa_build_plot (cast `/Game/Prototyping/Blueprints/Building/BPA_BuildPlot` _hitactor)
          (:`then`
            (bind _returnvalue (`AddComponent|NODE_AddStaticMeshComponent-0` :`self` _asbpa_build_plot :`RelativeTransform` (`KismetMathLibrary.Conv_VectorToTransform` _impactnormal)))
            (`StaticMeshComponent.SetStaticMesh` _returnvalue "/Engine/BasicShapes/Cube.Cube")
            (`PrimitiveComponent.SetMaterial` _returnvalue 0 "/Game/Prototyping/Blueprints/Building/M_BuildPreview.M_BuildPreview"))
          (:`CastFailed`
            (`KismetSystemLibrary.PrintString` "Miss")))))))

(fn `UserConstructionScript`)