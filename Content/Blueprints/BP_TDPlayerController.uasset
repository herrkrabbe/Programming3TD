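; BP_TDPlayerController is the player controller that sets up the game UI and the wave start button.
; On BeginPlay it creates the HUD and start-wave button widgets, stores both references and adds them to the viewport.
; Its WaveEnded event tells the button widget to reappear when a wave finishes.
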(event `self.ReceiveBeginPlay`
  (bind _returnvalue (`|CreateWidget` "/Game/HUD/WBP_HUD.WBP_HUD_C" self))
  (bind _output_get (set `self.HUD_Widget` _returnvalue))
  (`UserWidget.AddToViewport` _output_get 0)
  (bind _returnvalue_2 (`|CreateWidget` "/Game/HUD/WBP_StartWaveButton.WBP_StartWaveButton_C" self))
  (bind _output_get_2 (set `self.Button_Widget` _returnvalue_2))
  (`UserWidget.AddToViewport` _output_get_2 0))

(event `self.WaveEnded`
  (`/Game/HUD/WBP_StartWaveButton.Button Reappear` (`self.Button_Widget`)))

(fn `UserConstructionScript`)